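; Blueprint interface for the JigSInventory multiplayer inventory component, declaring callbacks for inventory events.
; Callbacks cover items added, removed, moved, dropped, consumed or picked up and equipped, plus container swaps, chamber UID updates and drop requests.
; Items and containers are identified by UIDs, names and info data, and a getter exposes the loot widget.
; Nearly every function returns a boolean, with no logic in the interface itself.
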(fn JigMPonMainContainerItemRemoved
  (params (FromContainerUID :type Integer) (ItemUID :type Integer) (ContainerName :type Name) (ItemRemovedInfo :type Rep%20Item%20Info%20Structure))
  (return false))

(fn JigMPonMainContainerItemAdded
  (params (ToContainerUID :type Integer) (ItemUID :type Integer) (ToContainerName :type Name) (ItemInfo :type Rep%20Item%20Info%20Structure) (FromMain :type Name))
  (return false 0))

(fn JigMPonPickupAdded
  (params (Info :type Rep%20Item%20Info%20Structure) (ItemUID :type Integer) (ToContainerUID :type Integer) (ToContainer :type Name))
  (return false))

(fn JigMPonPickupEquipped
  (params (ActorRef :type Actor%20Object%20Reference) (ToContainerName :type Name) (UID :type Integer) (ToContainerUID :type Integer) (Info :type Rep%20Item%20Info%20Structure))
  (return false))

(fn JigMPonRequestDropItem
  (params (ItemInfo :type Rep%20Item%20Info%20Structure) (ContainerName :type Name))
  (return 0))

(fn JigMPonItemConsumed
  (params (ConsumedItem :type Rep%20Item%20Info%20Structure) (Amount :type Integer) (Remaining :type Integer) (InsideOf :type Rep%20Item%20Info%20Structure) (FromContainer :type Name))
  (return false))

(fn JigMPonUpdateChamberUID
  (params (NewUID :type Integer))
  (return false))

(fn JigMPonTwoContainersSwap
  (params (FromContainer :type Name) (ToContainer :type Name))
  (return false))

(fn JigMPonItemMoved
  (params (ItemUID :type Integer) (FromContainerUID :type Integer) (ToContainerUID :type Integer))
  (return false))

(fn JigMPonItemAdded
  (params (ItemUID :type Integer) (FromContainerUID :type Integer) (ToContainerUID :type Integer) (FromComponent :type BP%20Jig%20Multiplayer%20Object%20Reference))
  (return false))

(fn JigMPonItemRemoved
  (params (ItemUID :type Integer) (FromContainerUID :type Integer) (ToContainerUID :type Integer) (ToComponent :type BP%20Jig%20Multiplayer%20Object%20Reference))
  (return false))

(fn JigMPonItemDropped
  (params (ItemUID :type Integer) (FromContainerUID :type Integer) (ActorRef :type Actor%20Object%20Reference))
  (return false))

(fn JigMPonContainersSwap
  (params (Container1 :type JSI%20Container%20Object%20Reference) (Container2 :type JSI%20Container%20Object%20Reference))
  (return false))

(fn JigMPGetLootWidget
  (return 0 false))