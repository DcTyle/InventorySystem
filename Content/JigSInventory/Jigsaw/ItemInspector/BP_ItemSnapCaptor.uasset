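; Capture actor that renders inventory and action bar images of Jigsaw items from their 3D meshes.
; SetJigitem applies mesh, pose and FOV from game state snap info; custom framing and live capture are also supported.
; InstallAttachments spawns equipped attachments from a data table, socketing them to the item or parent attachments.
; A show-only SceneCapture2D renders into slot-sized render targets, optionally cached and shared by ItemID.
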(event EventBeginPlay
  (Variables|/Script/Engine.SceneCaptureComponent2D|SetFOVAngle (Variables|Default|GetSceneCaptureComponent2D) (Variables|Default|GetInitialFOV))
  (Variables|/Script/Engine.SceneCaptureComponent|SetMaxViewDistanceOverride (Variables|Default|GetSceneCaptureComponent2D) 1e+03))

(fn ConstructionScript
  (Variables|/Script/Engine.SceneCaptureComponent|SetShowOnlyActors (Variables|Default|GetSceneCaptureComponent2D) (Utilities|Array|MakeArray self)))

(fn SetJigitem
  (params (ItemRef :type JSI%20Slot%20Object%20Reference))
  ;[0.05208 0.05208 0.05208] Set the mesh to inspect
  (bind _output_get (Variables|Default|SetItemToInspect ItemRef))
  (LocalVariables|SetIsActionBarItem (CallFunction|IsActionbar _output_get))
  (Utilities|FlowControl|Sequence
    (:then_0
      (bind _outputpin (Utilities|MGetSnapInfo (Default|GetItemID _output_get))
        (:true
          (if (.UseAsInventoryImage (Utilities|Struct|BreakS_ItemInspectInfo _outputpin))
            (Utilities|FlowControl|Sequence
              (:then_0
                (Components|StaticMesh|SetStaticMesh (Variables|Default|GetStaticMesh) 0)
                (Class|SkinnedMeshComponent|SetSkeletalMesh (Variables|Default|GetSkeletalMesh) 0 false)
                (Transformation|SetRelativeLocationAndRotation (Variables|Default|GetSkeletalMesh) (Math|Vector|SelectVector (.ActionBarLoc (Utilities|Struct|BreakS_ItemInspectInfo _outputpin)) (.InspectLoc (Utilities|Struct|BreakS_ItemInspectInfo _outputpin)) (LocalVariables|GetIsActionBarItem)) (Math|Rotator|SelectRotator (.ActionBarRot (Utilities|Struct|BreakS_ItemInspectInfo _outputpin)) (.InspectRot (Utilities|Struct|BreakS_ItemInspectInfo _outputpin)) (LocalVariables|GetIsActionBarItem)) false true))
              (:then_1
                (Utilities|IsValid (.SKMeshToInspect (Utilities|Struct|BreakS_ItemInspectInfo _outputpin))
                  (:Is%20Valid
                    (Class|SkinnedMeshComponent|SetSkeletalMesh (Variables|Default|GetSkeletalMesh) (.SKMeshToInspect (Utilities|Struct|BreakS_ItemInspectInfo _outputpin)) false))
                  (:Is%20Not%20Valid
                    (Components|StaticMesh|SetStaticMesh (Variables|Default|GetStaticMesh) (.SMMeshToInspect (Utilities|Struct|BreakS_ItemInspectInfo _outputpin)))))
                (Variables|/Script/Engine.SceneCaptureComponent2D|SetFOVAngle (Variables|Default|GetSceneCaptureComponent2D) (Math|Float|SelectFloat (.ActionBarFOV (Utilities|Struct|BreakS_ItemInspectInfo _outputpin)) (.InitialFOV (Utilities|Struct|BreakS_ItemInspectInfo _outputpin)) (LocalVariables|GetIsActionBarItem)))
                (return true (.ShareRenderTargetWithSimilarItems (Utilities|Struct|BreakS_ItemInspectInfo _outputpin)))))
            (else
              (return false false))))
        (:false
          (return false false))))
    (:then_1
      (return false false))))

(fn GetSnap
  (params (ShareRTarget :type Boolean))
  (bind _itemtoinspect (Variables|Default|GetItemToInspect))
  (bind _scenecapturecomponent2d (Variables|Default|GetSceneCaptureComponent2D))
  (bind _result (CallFunction|IsActionbar _itemtoinspect))
  (bind _slotdimension (CallFunction|GetDefaultDim _itemtoinspect))
  (bind _returnvalue (* _slotdimension 9e+01))
  (bind _returnvalue_2 (select _result "(X=128.000000,Y=128.000000)" _returnvalue))
  (bind (_x _y) (Math|Vector2D|BreakVector2D _returnvalue_2))
  (if ShareRTarget
    (bind _output_get (LocalVariables|SetRenderTarg (.Value (Utilities|Map|Find (Variables|Default|GetCreatedRenderTargets) (.ItemID (Utilities|Struct|BreakFItemInfo (Variables|/Game/JigSInventory/Jigsaw/Widgets/JSI_Slot.JSI_Slot_C|GetItemInfo _itemtoinspect)))))))
    (Utilities|IsValid _output_get
      (:Is%20Valid
        (return (LocalVariables|GetRenderTarg) true))
      (:Is%20Not%20Valid
        (LocalVariables|SetSaveRTarget true))))
  (bind _returnvalue_3 (Rendering|CreateRenderTarget2D (Math|Float|Truncate _x) (Math|Float|Truncate _y) "RTF_RGBA16f"))
  (bind _output_get_2 (LocalVariables|SetRenderTarg _returnvalue_3))
  (Variables|/Script/Engine.SceneCaptureComponent2D|SetTextureTarget (Variables|Default|GetSceneCaptureComponent2D) _output_get_2)
  (Rendering|SceneCapture|CaptureScene _scenecapturecomponent2d :!class /Script/Engine.SceneCaptureComponent2D)
  (Variables|/Script/Engine.SceneCaptureComponent2D|SetTextureTarget _scenecapturecomponent2d 0)
  (Utilities|FlowControl|Sequence
    (:then_0
      (if (LocalVariables|GetSaveRTarget)
        (Utilities|Map|Add (Variables|Default|GetCreatedRenderTargets) (Utilities|Struct|BreakFItemInfo (Variables|/Game/JigSInventory/Jigsaw/Widgets/JSI_Slot.JSI_Slot_C|GetItemInfo (Variables|Default|GetItemToInspect))) (LocalVariables|GetRenderTarg))))
    (:then_1
      (return (LocalVariables|GetRenderTarg) false))))

(fn UpdateSnap
  (params (ItemRef :type JSI%20Slot%20Object%20Reference) (TextureTarget :type Texture%20Render%20Target%202D%20Object%20Reference))
  (bind _scenecapturecomponent2d (Variables|Default|GetSceneCaptureComponent2D))
  (CallFunction|SetJigitem ItemRef)
  (bind _output_get (Variables|/Script/Engine.SceneCaptureComponent2D|SetTextureTarget _scenecapturecomponent2d TextureTarget))
  (Rendering|SceneCapture|CaptureScene _scenecapturecomponent2d :!class /Script/Engine.SceneCaptureComponent2D)
  (Variables|/Script/Engine.SceneCaptureComponent2D|SetTextureTarget _scenecapturecomponent2d 0)
  (return _output_get))

(fn InstallAttachments
  (params (JigItem :type JSI%20Slot%20Object%20Reference))
  (bind _containerref (Default|GetContainerOneRef JigItem))
  (Utilities|Array|Clear (LocalVariables|GetAllAttachments))
  (Utilities|IsValid _containerref
    (:Is%20Valid
      (bind _containers (Class|JSISpecialWidgetInterface|GetListOfContainers(Message) _containerref))
      (for _array_element _containers
        (if (Default|IsEquipTo? _array_element)
          (Default|DeepGettAllItems _array_element (LocalVariables|GetAllAttachments))))
      (for _array_element_2 (LocalVariables|GetAllAttachments)
        (LocalVariables|SetCurrentJig _array_element_2)
        (bind _returnvalue (Utilities|GetDataTableRow "/Game/JigSInventory/Demo/Pickups/LocalAttachments/DT_LocalAttachments.DT_LocalAttachments" (Default|GetItemID _array_element_2))
          (:then
            (LocalVariables|SetLocalInfo _returnvalue)
            (bind _returnvalue_2 (Game|SpawnActorfromClass (.AttachmentClass (Utilities|Struct|BreakLocalAttachmentInfo _returnvalue)) (Math|Transform|MakeTransform (Transformation|GetActorLocation) "0, 0, 0" "1,1,1") "Undefined" 0 0))
            (Utilities|IsValid _returnvalue_2
              (:Is%20Valid
                (LocalVariables|SetSpawnedItem _returnvalue_2)
                (Utilities|Array|Add (Variables|Default|GetCurrentAttachments) _returnvalue_2)
                (Default|JigSetAttachmentInfo _returnvalue_2 (Default|GetUniqueID (LocalVariables|GetCurrentJig)) (LocalVariables|GetLocalInfo))
                (LocalVariables|SetParentUID (Default|GetSlotMotherUID (Variables|/Game/JigSInventory/Jigsaw/Widgets/JSI_Slot.JSI_Slot_C|GetContainerMother (LocalVariables|GetCurrentJig)) false false))
                (if (== (LocalVariables|GetParentUID) (Default|GetUniqueID JigItem))
                  (bind _comp (Class|BPWeaponAttachments|JigGetPrimitiveComponent(Message) (LocalVariables|GetSpawnedItem)))
                  (Transformation|AttachComponentToComponent _comp (CallFunction|GetActiveComponent) (.AttachToSocket (Utilities|Struct|BreakLocalAttachmentInfo (LocalVariables|GetLocalInfo))) "SnapToTarget" "SnapToTarget" "KeepWorld" true)
                  (else
                    ;[0 0.2186 1] Ex: an laser sight on a handguard, things that are installed on other attachments instead of the weapon itself.
                    (bind _array_element_3 (Utilities|Array|ForEachLoopwithBreak (Variables|Default|GetCurrentAttachments) :!label _label)
                      (:LoopBody
                        (bind _uid (Class|BPWeaponAttachments|JigGetAttachmentInfo(Message) _array_element_3))
                        (if (== _uid (LocalVariables|GetParentUID))
                          (Utilities|FlowControl|Sequence
                            (:then_0
                              (bind _comp_2 (Class|BPWeaponAttachments|JigGetPrimitiveComponent(Message) _array_element_3))
                              (bind _comp_3 (Class|BPWeaponAttachments|JigGetPrimitiveComponent(Message) (LocalVariables|GetSpawnedItem)))
                              (Transformation|AttachComponentToComponent _comp_3 _comp_2 (CallFunction|GetAttachSocketbyinContainerIndex (LocalVariables|GetLocalInfo) (Default|GetContainerIndex (Variables|/Game/JigSInventory/Jigsaw/Widgets/JSI_Slot.JSI_Slot_C|GetContainerMother (LocalVariables|GetCurrentJig)))) "SnapToTarget" "SnapToTarget" "KeepWorld" true))
                            (:then_1
                              (goto _label Break)))))))))))))
      (for _array_element_4 (Variables|Default|GetCurrentAttachments)
        (bind _comp_4 (Class|BPWeaponAttachments|JigGetPrimitiveComponent(Message) _array_element_4))
        (Rendering|Components|SetLightingChannels _comp_4 false true false)
        (Utilities|Array|AppendArray (Variables|/Script/Engine.SceneCaptureComponent|GetShowOnlyActors (Variables|Default|GetSceneCaptureComponent2D)) (Variables|Default|GetCurrentAttachments))))))

(fn ClearAttachments
  (bind _scenecapturecomponent2d (Variables|Default|GetSceneCaptureComponent2D))
  (bind _currentattachments (Variables|Default|GetCurrentAttachments))
  (bind _showonlyactors (Variables|/Script/Engine.SceneCaptureComponent|GetShowOnlyActors _scenecapturecomponent2d))
  (Utilities|Array|Clear _showonlyactors)
  (Utilities|Array|Add _showonlyactors self)
  (bind _arrayelement (Utilities|Array|ReverseforEachLoop _currentattachments)
    (:LoopBody
      (Actor|DestroyActor _arrayelement))
    (:Completed
      (Utilities|Array|Clear _currentattachments))))

(fn IsActionbar
  (params (ItemRef :type JSI%20Slot%20Object%20Reference))
  (return (Variables|/Game/JigSInventory/Jigsaw/Widgets/JSIContainer.JSIContainer_C|GetIsActionbar (Variables|/Game/JigSInventory/Jigsaw/Widgets/JSI_Slot.JSI_Slot_C|GetContainerMother ItemRef))))

(fn GetInitValues
  (bind _skeletalmesh (Variables|Default|GetSkeletalMesh))
  (return (Transformation|GetRelativeTransform (select (Utilities|IsValid (Variables|/Script/Engine.SkinnedMeshComponent|GetSkeletalMesh _skeletalmesh)) _skeletalmesh (Variables|Default|GetStaticMesh))) (Variables|/Script/Engine.SceneCaptureComponent2D|GetFOVAngle (Variables|Default|GetSceneCaptureComponent2D))))

(fn GetDefaultDim
  (params (Target :type JSI%20Slot%20Object%20Reference))
  (bind _slotdimension (Default|GetSlotDim Target))
  (bind (_x _y) (Math|Vector2D|BreakVector2D _slotdimension))
  (if (and (!= _x _y) (not (CallFunction|IsActionbar Target)))
    (bind _returnvalue (Utilities|GetDataTableRow (Default|GetDtRef Target) (Default|GetItemID Target))
      (:then
        (return (Utilities|Struct|BreakFItemInfo _returnvalue))))
    (else
      (return _slotdimension))))

(fn GetSnapNoCapture
  (params (Item :type JSI%20Slot%20Object%20Reference) (ShareRTarget :type Boolean))
  (bind _result (CallFunction|IsActionbar Item))
  (bind _slotdimension (CallFunction|GetDefaultDim Item))
  (bind _returnvalue (* _slotdimension 6e+01))
  (bind _returnvalue_2 (select _result "(X=128.000000,Y=128.000000)" _returnvalue))
  (bind (_x _y) (Math|Vector2D|BreakVector2D _returnvalue_2))
  (if ShareRTarget
    (bind _output_get (LocalVariables|SetRenderTarg (.Value (Utilities|Map|Find (Variables|Default|GetCreatedRenderTargets) (.ItemID (Utilities|Struct|BreakFItemInfo (Variables|/Game/JigSInventory/Jigsaw/Widgets/JSI_Slot.JSI_Slot_C|GetItemInfo Item)))))))
    (Utilities|IsValid _output_get
      (:Is%20Valid
        (return (LocalVariables|GetRenderTarg) true))
      (:Is%20Not%20Valid
        (LocalVariables|SetSaveRTarget true))))
  (bind _returnvalue_3 (Rendering|CreateRenderTarget2D (Math|Float|Truncate _x) (Math|Float|Truncate _y) "RTF_RGBA16f"))
  (LocalVariables|SetRenderTarg _returnvalue_3)
  (Utilities|FlowControl|Sequence
    (:then_0
      (if (LocalVariables|GetSaveRTarget)
        (Utilities|Map|Add (Variables|Default|GetCreatedRenderTargets) (.ItemID (Utilities|Struct|BreakFItemInfo (Variables|/Game/JigSInventory/Jigsaw/Widgets/JSI_Slot.JSI_Slot_C|GetItemInfo Item))) (LocalVariables|GetRenderTarg))))
    (:then_1
      (return (LocalVariables|GetRenderTarg) false))))

(fn CapturefromTarget
  (params (TextureTarget :type Texture%20Render%20Target%202D%20Object%20Reference))
  (bind _scenecapturecomponent2d (Variables|Default|GetSceneCaptureComponent2D))
  (Variables|/Script/Engine.SceneCaptureComponent2D|SetTextureTarget (Variables|Default|GetSceneCaptureComponent2D) TextureTarget)
  (Rendering|SceneCapture|CaptureScene _scenecapturecomponent2d :!class /Script/Engine.SceneCaptureComponent2D)
  (Variables|/Script/Engine.SceneCaptureComponent2D|SetTextureTarget _scenecapturecomponent2d 0))

(fn IsLocked
  (return (Variables|Default|GetIsLocked?)))

(fn SetLocked
  (params (IsLocked? :type Boolean))
  (Variables|Default|SetIsLocked? IsLocked?))

(fn SetJigitemCustom
  (params (ItemRef :type JSI%20Slot%20Object%20Reference) (Location :type Vector) (Rotation :type Rotator) (FOV :type Float%20%28single-precision%29))
  ;[0.05208 0.05208 0.05208] Set the mesh to inspect
  (bind _output_get (Variables|Default|SetItemToInspect ItemRef))
  (Utilities|FlowControl|Sequence
    (:then_0
      (bind _outputpin (Utilities|MGetSnapInfo (Default|GetItemID _output_get))
        (:true
          (if (.UseAsInventoryImage (Utilities|Struct|BreakS_ItemInspectInfo _outputpin))
            (Utilities|FlowControl|Sequence
              (:then_0
                (CallFunction|ClearAttachments)
                (Components|StaticMesh|SetStaticMesh (Variables|Default|GetStaticMesh) 0)
                (Class|SkinnedMeshComponent|SetSkeletalMesh (Variables|Default|GetSkeletalMesh) 0 false)
                (Transformation|SetRelativeLocationAndRotation (Variables|Default|GetSkeletalMesh) Location Rotation false true))
              (:then_1
                (Utilities|IsValid (.SKMeshToInspect (Utilities|Struct|BreakS_ItemInspectInfo _outputpin))
                  (:Is%20Valid
                    (Class|SkinnedMeshComponent|SetSkeletalMesh (Variables|Default|GetSkeletalMesh) (.SKMeshToInspect (Utilities|Struct|BreakS_ItemInspectInfo _outputpin)) false))
                  (:Is%20Not%20Valid
                    (Components|StaticMesh|SetStaticMesh (Variables|Default|GetStaticMesh) (.SMMeshToInspect (Utilities|Struct|BreakS_ItemInspectInfo _outputpin)))))
                (Variables|/Script/Engine.SceneCaptureComponent2D|SetFOVAngle (Variables|Default|GetSceneCaptureComponent2D) FOV)
                (return true (.ShareRenderTargetWithSimilarItems (Utilities|Struct|BreakS_ItemInspectInfo _outputpin)))))
            (else
              (return false false))))
        (:false
          (return false false))))
    (:then_1
      (return false false))))

(fn ToggleCapture
  (params (IsActive :type Boolean) (Texture%20Target :type Texture%20Render%20Target%202D%20Object%20Reference))
  (Variables|/Script/Engine.SceneCaptureComponent|SetbCaptureEveryFrame (Variables|Default|GetSceneCaptureComponent2D) IsActive)
  (Variables|/Script/Engine.SceneCaptureComponent2D|SetTextureTarget (Variables|Default|GetSceneCaptureComponent2D) Texture%20Target))

(fn GetActiveComponent
  (Utilities|IsValid (Variables|/Script/Engine.StaticMeshComponent|GetStaticMesh (Variables|Default|GetStaticMesh))
    (:Is%20Valid
      (return (Variables|Default|GetStaticMesh)))
    (:Is%20Not%20Valid
      (return (Variables|Default|GetSkeletalMesh)))))

(fn GetAttachSocketbyinContainerIndex
  (params (Info :type Local%20Attachment%20Info%20Structure%20%28by%20ref%29) (InContainerIndex :type Integer))
  (bind (_attachtosocket _attachtosocketbycontainerindex) (Utilities|Struct|BreakLocalAttachmentInfo Info))
  ;[1 1 1] In container index: Take a handguard for example, a laser sight could be installed to the left or the right side, so we determine the socket based on InContainerIndex.
  ; This depends on how you setup your special container.
  (Utilities|FlowControl|Sequence
    (:then_0
      (for _array_element _attachtosocketbycontainerindex
        (if (== (.Index (Utilities|Struct|BreakS_LocalAttContainerIndexSocket _array_element)) InContainerIndex)
          (return (.SocketName (Utilities|Struct|BreakS_LocalAttContainerIndexSocket _array_element))))))
    (:then_1
      (return _attachtosocket))))