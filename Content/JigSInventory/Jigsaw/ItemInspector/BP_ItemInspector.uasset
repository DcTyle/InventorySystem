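; Item inspector actor that renders an inventory item to a render target through a show-only scene capture, with spring-arm rotation and FOV zoom.
; Mesh, transform and zoom limits come from game-state inspect info looked up by item ID.
; Equipped attachments spawn from DT_LocalAttachments, are reused or destroyed by UID, and snap to sockets on the item or parent attachments, using lighting channel 1.
; Capture runs on demand or every frame while active.
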(event EventBeginPlay
  ;[0.02604 0.02604 0.02604] Begin play
  (Components|Activation|Deactivate (Variables|Default|GetSceneCaptureComponent2D))
  (Variables|/Script/Engine.SceneCaptureComponent2D|SetFOVAngle (Variables|Default|GetSceneCaptureComponent2D) (Variables|Default|GetInitialFOV))
  (Variables|/Script/Engine.SceneCaptureComponent|SetMaxViewDistanceOverride (Variables|Default|GetSceneCaptureComponent2D) 1e+03))

(event EventEndPlay
  (params (EndPlayReason :type EEndPlayReason%20Enum :default "Destroyed"))
  (bind _currentattachments (Variables|Default|GetCurrentAttachments))
  ;[0.005208 0.005208 0.005208] End play
  (Variables|/Game/JigSInventory/Jigsaw/Widgets/JSI_Slot.JSI_Slot_C|SetInspectorWidget (Variables|Default|GetItemToInspect) 0)
  (Class|KismetRenderingLibrary|ReleaseRenderTarget2D (Variables|Default|GetRenderT))
  (bind _arrayelement (Utilities|Array|ReverseforEachLoop _currentattachments)
    (:LoopBody
      (Actor|DestroyActor _arrayelement))
    (:Completed
      (Utilities|Array|Clear _currentattachments))))

(fn ConstructionScript
  (Variables|/Script/Engine.SceneCaptureComponent|SetShowOnlyActors (Variables|Default|GetSceneCaptureComponent2D) (Utilities|Array|MakeArray self)))

(fn SetItemtoInspect
  (params (ItemRef :type JSI%20Slot%20Object%20Reference))
  (bind _staticmesh (Variables|Default|GetStaticMesh))
  (bind _skeletalmesh (Variables|Default|GetSkeletalMesh))
  (Utilities|FlowControl|Sequence
    (:then_0
      ;[1 1 1] Create the render target
      (bind _returnvalue (Rendering|CreateRenderTarget2D 512 512 "RTF_RGBA16f"))
      (bind _output_get (Variables|/Script/Engine.SceneCaptureComponent2D|SetTextureTarget (Variables|Default|GetSceneCaptureComponent2D) _returnvalue))
      (Variables|Default|SetRenderT _output_get))
    (:then_1
      ;[0.05208 0.05208 0.05208] Set the mesh to inspect
      (bind _output_get_2 (Variables|Default|SetItemToInspect ItemRef))
      (Utilities|FlowControl|Sequence
        (:then_0
          (bind _out_row (Utilities|MGetInspectInfo (Default|GetItemID _output_get_2))
            (:Row%20Found
              (Utilities|FlowControl|Sequence
                (:then_0
                  (Components|StaticMesh|SetStaticMesh (Variables|Default|GetStaticMesh) 0)
                  (Class|SkinnedMeshComponent|SetSkeletalMesh (Variables|Default|GetSkeletalMesh) 0 false))
                (:then_1
                  (Utilities|IsValid (.SKMeshToInspect (Utilities|Struct|BreakS_ItemInspectInfo _out_row))
                    (:Is%20Valid
                      (Class|SkinnedMeshComponent|SetSkeletalMesh _skeletalmesh (.SKMeshToInspect (Utilities|Struct|BreakS_ItemInspectInfo _out_row)) false)
                      (Transformation|SetRelativeLocationAndRotation _skeletalmesh (.InspectLoc (Utilities|Struct|BreakS_ItemInspectInfo _out_row)) (.InspectRot (Utilities|Struct|BreakS_ItemInspectInfo _out_row)) false true))
                    (:Is%20Not%20Valid
                      (Components|StaticMesh|SetStaticMesh _staticmesh (.SMMeshToInspect (Utilities|Struct|BreakS_ItemInspectInfo _out_row)))
                      (Transformation|SetRelativeLocationAndRotation _staticmesh (.InspectLoc (Utilities|Struct|BreakS_ItemInspectInfo _out_row)) (.InspectRot (Utilities|Struct|BreakS_ItemInspectInfo _out_row)) false true)))
                  (Variables|Default|SetMaxZoomInFOV (.MaZoomInFOV (Utilities|Struct|BreakS_ItemInspectInfo _out_row)))
                  (Variables|Default|SetMaxZoomOutFOV (.MaZoomOutFOV (Utilities|Struct|BreakS_ItemInspectInfo _out_row)))
                  (Variables|/Script/Engine.SceneCaptureComponent2D|SetFOVAngle (Variables|Default|GetSceneCaptureComponent2D) (.InitialFOV (Utilities|Struct|BreakS_ItemInspectInfo _out_row))))))
            (:RowNotFound
              (Development|PrintString (Utilities|String|ToString(Text) (Utilities|Text|FormatText "Could not find {ItemID} in DT_ItemInspector data table" (Default|GetItemID _output_get_2))) true true "(R=1.000000,G=0.000000,B=0.000000,A=1.000000)" 5.0))))
        (:then_1
          (Rendering|SceneCapture|CaptureScene (Variables|Default|GetSceneCaptureComponent2D) :!class /Script/Engine.SceneCaptureComponent2D))))))

(fn SetMeshRotation
  (params (XYRot :type Vector%202D%20Structure))
  (Transformation|AddLocalRotation (Variables|Default|GetSpringArm) (Math|Rotator|MakeRotator 0.0 (.y XYRot) (* (.x XYRot) -1.0)) false false))

(fn OnZoomOut
  (bind _scenecapturecomponent2d (Variables|Default|GetSceneCaptureComponent2D))
  (Variables|/Script/Engine.SceneCaptureComponent2D|SetFOVAngle _scenecapturecomponent2d (Math|Float|Clamp(Float) (+ (Variables|/Script/Engine.SceneCaptureComponent2D|GetFOVAngle _scenecapturecomponent2d) 5.0) (Variables|Default|GetMaxZoomInFOV) (Variables|Default|GetMaxZoomOutFOV)))
  (if (not (Components|Activation|IsActive _scenecapturecomponent2d))
    (Rendering|SceneCapture|CaptureScene (Variables|Default|GetSceneCaptureComponent2D) :!class /Script/Engine.SceneCaptureComponent2D)))

(fn OnZoomin
  (bind _scenecapturecomponent2d (Variables|Default|GetSceneCaptureComponent2D))
  (Variables|/Script/Engine.SceneCaptureComponent2D|SetFOVAngle _scenecapturecomponent2d (Math|Float|Clamp(Float) (+ (Variables|/Script/Engine.SceneCaptureComponent2D|GetFOVAngle _scenecapturecomponent2d) -5.0) (Variables|Default|GetMaxZoomInFOV) (Variables|Default|GetMaxZoomOutFOV)))
  (if (not (Components|Activation|IsActive _scenecapturecomponent2d))
    (Rendering|SceneCapture|CaptureScene (Variables|Default|GetSceneCaptureComponent2D) :!class /Script/Engine.SceneCaptureComponent2D)))

(fn GetRenderTarget
  (return (Variables|Default|GetRenderT)))

(fn UpdateLocandRot
  (params (NewLocation :type Vector) (NewRotation :type Rotator) (FOVAngle :type Float%20%28single-precision%29))
  (Transformation|SetRelativeLocationAndRotation (Variables|Default|GetStaticMesh) NewLocation NewRotation false true)
  (Variables|/Script/Engine.SceneCaptureComponent2D|SetFOVAngle (Variables|Default|GetSceneCaptureComponent2D) FOVAngle)
  (Rendering|SceneCapture|CaptureScene (Variables|Default|GetSceneCaptureComponent2D) :!class /Script/Engine.SceneCaptureComponent2D))

(fn GetInitValues
  (bind _skeletalmesh (Variables|Default|GetSkeletalMesh))
  (return (Transformation|GetRelativeTransform (select (Utilities|IsValid (Variables|/Script/Engine.SkinnedMeshComponent|GetSkeletalMesh _skeletalmesh)) _skeletalmesh (Variables|Default|GetStaticMesh))) (Variables|/Script/Engine.SceneCaptureComponent2D|GetFOVAngle (Variables|Default|GetSceneCaptureComponent2D))))

(fn SetCaptorActiveState
  (params (IsActive :type Boolean))
  (bind _scenecapturecomponent2d (Variables|Default|GetSceneCaptureComponent2D))
  (Components|Activation|SetActive _scenecapturecomponent2d IsActive false)
  (Variables|/Script/Engine.SceneCaptureComponent|SetbCaptureEveryFrame _scenecapturecomponent2d IsActive))

(fn GetAttachSocketbyinContainerIndex
  (params (Info :type Local%20Attachment%20Info%20Structure%20%28by%20ref%29) (InContainerIndex :type Integer))
  (bind (_attachtosocket _attachtosocketbycontainerindex) (Utilities|Struct|BreakLocalAttachmentInfo Info))
  ;[1 1 1] In container index: Take a handguard for example, a laser sight could be installed to the left or the right side, so we determine the socket based on InContainerIndex.
  ; This depends on how you setup your special container.
  (Utilities|FlowControl|Sequence
    (:then_0
      (for _array_element _attachtosocketbycontainerindex
        (if (== (.Index (Utilities|Struct|BreakS_LocalAttContainerIndexSocket _array_element)) InContainerIndex)
          (return (.SocketName (Utilities|Struct|BreakS_LocalAttContainerIndexSocket _array_element))))))
    (:then_1
      (return _attachtosocket))))

(fn GetActiveComponent
  (Utilities|IsValid (Variables|/Script/Engine.StaticMeshComponent|GetStaticMesh (Variables|Default|GetStaticMesh))
    (:Is%20Valid
      (return (Variables|Default|GetStaticMesh)))
    (:Is%20Not%20Valid
      (return (Variables|Default|GetSkeletalMesh)))))

(fn ClearAttachments
  (bind _scenecapturecomponent2d (Variables|Default|GetSceneCaptureComponent2D))
  (bind _currentattachments (Variables|Default|GetCurrentAttachments))
  (bind _showonlyactors (Variables|/Script/Engine.SceneCaptureComponent|GetShowOnlyActors _scenecapturecomponent2d))
  (Utilities|Array|Clear _showonlyactors)
  (Utilities|Array|Add _showonlyactors self)
  (bind _arrayelement (Utilities|Array|ReverseforEachLoop _currentattachments)
    (:LoopBody
      (Actor|DestroyActor _arrayelement))
    (:Completed
      (Utilities|Array|Clear _currentattachments))))

(fn InstallAttachments
  (params (JigItem :type JSI%20Slot%20Object%20Reference))
  (bind _containerref (Default|GetContainerOneRef JigItem))
  (bind _currentattachments (Variables|Default|GetCurrentAttachments))
  (Utilities|Array|Clear (LocalVariables|GetAllAttachments))
  (Utilities|IsValid _containerref
    (:Is%20Valid
      (bind _containers (Class|JSISpecialWidgetInterface|GetListOfContainers(Message) _containerref))
      (for _array_element _containers
        (if (Default|IsEquipTo? _array_element)
          (Default|DeepGettAllItems _array_element (LocalVariables|GetAllAttachments))))
      (for _array_element_2 (LocalVariables|GetAllAttachments)
        (bind _output_get (LocalVariables|SetCurrentJig _array_element_2))
        (Utilities|Array|Add (LocalVariables|GetAllJigUIDs) (Default|GetUniqueID _output_get))
        (bind _attachment (CallFunction|FindLocalAttachmentbyUID (Default|GetUniqueID _output_get)))
        (bind _output_get_2 (LocalVariables|SetSpawnedItem _attachment))
        (bind _attachmentinfo (Class|BPWeaponAttachments|JigGetAttachmentInfo(Message) _output_get_2))
        (LocalVariables|SetLocalInfo _attachmentinfo)
        (Utilities|IsValid _output_get_2
          (:Is%20Valid
            (LocalVariables|SetParentUID (Default|GetSlotMotherUID (Variables|/Game/JigSInventory/Jigsaw/Widgets/JSI_Slot.JSI_Slot_C|GetContainerMother (LocalVariables|GetCurrentJig)) false false) :!label _label)
            (if (== (LocalVariables|GetParentUID) (Default|GetUniqueID JigItem))
              (bind _comp (Class|BPWeaponAttachments|JigGetPrimitiveComponent(Message) (LocalVariables|GetSpawnedItem)))
              (Transformation|AttachComponentToComponent _comp (CallFunction|GetActiveComponent) (.AttachToSocket (Utilities|Struct|BreakLocalAttachmentInfo (LocalVariables|GetLocalInfo))) "SnapToTarget" "SnapToTarget" "KeepWorld" true)
              (else
                ;[0 0.2186 1] Ex: an laser sight on a handguard, things that are installed on other attachments instead of the weapon itself.
                (bind _attachment_2 (CallFunction|FindLocalAttachmentbyUID (LocalVariables|GetParentUID)))
                (Utilities|IsValid _attachment_2
                  (:Is%20Valid
                    (bind _comp_2 (Class|BPWeaponAttachments|JigGetPrimitiveComponent(Message) _attachment_2))
                    (bind _comp_3 (Class|BPWeaponAttachments|JigGetPrimitiveComponent(Message) (LocalVariables|GetSpawnedItem)))
                    (Transformation|AttachComponentToComponent _comp_3 _comp_2 (CallFunction|GetAttachSocketbyinContainerIndex (LocalVariables|GetLocalInfo) (Default|GetContainerIndex (Variables|/Game/JigSInventory/Jigsaw/Widgets/JSI_Slot.JSI_Slot_C|GetContainerMother (LocalVariables|GetCurrentJig)))) "SnapToTarget" "SnapToTarget" "KeepWorld" true))))))
          (:Is%20Not%20Valid
            (bind _returnvalue (Utilities|GetDataTableRow "/Game/JigSInventory/Demo/Pickups/LocalAttachments/DT_LocalAttachments.DT_LocalAttachments" (Default|GetItemID _array_element_2))
              (:then
                (LocalVariables|SetLocalInfo _returnvalue)
                (bind _returnvalue_2 (Game|SpawnActorfromClass (.AttachmentClass (Utilities|Struct|BreakLocalAttachmentInfo _returnvalue)) (Math|Transform|MakeTransform (Transformation|GetActorLocation) "0, 0, 0" "1,1,1") "Undefined" 0 0))
                (bind _output_get_3 (LocalVariables|SetSpawnedItem _returnvalue_2))
                (Utilities|IsValid _output_get_3
                  (:Is%20Valid
                    (Utilities|Array|Add (Variables|Default|GetCurrentAttachments) (LocalVariables|GetSpawnedItem))
                    (Default|JigSetAttachmentInfo (LocalVariables|GetSpawnedItem) (Default|GetUniqueID (LocalVariables|GetCurrentJig)) (LocalVariables|GetLocalInfo))
                    (Utilities|FlowControl|Sequence
                      (:then_0
                        (bind _comp_4 (Class|BPWeaponAttachments|JigGetPrimitiveComponent(Message) (LocalVariables|GetSpawnedItem)))
                        (Rendering|Components|SetLightingChannels _comp_4 false true false)
                        (Utilities|Array|Add (Variables|/Script/Engine.SceneCaptureComponent|GetShowOnlyActors (Variables|Default|GetSceneCaptureComponent2D)) (LocalVariables|GetSpawnedItem)))
                      (:then_1
                        (goto _label))))))))))
      ;[0.04688 0.04688 0.04688] Destroy non existing attachments
      (bind (_arrayindex _arrayelement) (Utilities|Array|ReverseforEachLoop _currentattachments)
        (:LoopBody
          (bind _uid (Class|BPWeaponAttachments|JigGetAttachmentInfo(Message) _arrayelement))
          (if (not (Utilities|Array|ContainsItem (LocalVariables|GetAllJigUIDs) _uid))
            (Utilities|Array|RemoveItem (Variables|/Script/Engine.SceneCaptureComponent|GetShowOnlyActors (Variables|Default|GetSceneCaptureComponent2D)) _arrayelement)
            (Actor|DestroyActor _arrayelement)
            (Utilities|Array|RemoveIndex _currentattachments _arrayindex)))))))

(fn FindLocalAttachmentbyUID
  (params (UID :type Integer))
  (for _array_element (Variables|Default|GetCurrentAttachments)
    (bind _uid (Class|BPWeaponAttachments|JigGetAttachmentInfo(Message) _array_element))
    (if (== _uid UID)
      (return _array_element)))
  (return 0))

(fn CaptureOneFrame
  (if (not (Variables|/Script/Engine.SceneCaptureComponent|GetbCaptureEveryFrame (Variables|Default|GetSceneCaptureComponent2D)))
    (Rendering|SceneCapture|CaptureScene (Variables|Default|GetSceneCaptureComponent2D) :!class /Script/Engine.SceneCaptureComponent2D)))